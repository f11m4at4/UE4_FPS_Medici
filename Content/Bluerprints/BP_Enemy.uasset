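; Enemy Blueprint that runs a simple state machine, switching on a State enum each Tick and printing the current state for debugging.
; Idle accumulates delta time until it passes a delay, then switches to Move, which feeds the unnormalized direction toward a Target actor into movement input.
; Attack, Damage and Die are empty stubs, nothing transitions out of Move, and Target is never assigned in these graphs.
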(event EventBeginPlay)

(event Collision|EventActorBeginOverlap
  (params (OtherActor :type Actor%20Object%20Reference)))

(event EventTick
  (params (DeltaSeconds :type Float%20%28single-precision%29))
  (bind _state (Variables|Default|Getstate))
  (Development|PrintString (Utilities|String|EnumtoString _state) true true "(R=0.000000,G=0.660000,B=1.000000,A=1.000000)" 0.0)
  (switch Utilities|FlowControl|Switch|SwitchonEEnemyState _state
    (:NewEnumerator0
      (CallFunction|IdleState))
    (:NewEnumerator1
      (CallFunction|MoveState))
    (:NewEnumerator2
      (CallFunction|AttackState))
    (:NewEnumerator3
      (CallFunction|DamageState))
    (:NewEnumerator4
      (CallFunction|DieState))))

(fn ConstructionScript)

(fn IdleState
  (bind _output_get (Variables|Default|SetCurrentTime (+ (Variables|Default|GetCurrentTime) (Utilities|Time|GetWorldDeltaSeconds))))
  (if (> _output_get (Variables|Default|GetIdleDelayTime))
    (Variables|Default|Setstate "NewEnumerator1")))

(fn MoveState
  (Pawn|Input|AddMovementInput (- (Transformation|GetActorLocation (Variables|Default|GetTarget)) (Transformation|GetActorLocation)) 1.0 false))

(fn AttackState)

(fn DamageState)

(fn DieState)